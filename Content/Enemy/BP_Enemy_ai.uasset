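; AI enemy character that spawns holding a gun, shoots the player and awards hit-location score when shot.
; Pawn sensing sets a blackboard flag on seeing the player.
; ShootPlayer rotates the enemy using the player's position, then, gated by CanAttach, spawns a projectile and applies damage directly.
; Head, body/arm and leg hitboxes each trigger ragdoll, delayed destruction and a matching game mode scoring call.
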(event OnSeePawn(PawnSensing)
  (params (Pawn :type Pawn%20Object%20Reference))
  (Utilities|Casting|CastToBP_FirstPersonCharacter Pawn)
  (AI|Components|Blackboard|SetValueasBool (AI|GetBlackboard (AI|GetAIController self)) (Utilities|Name|MakeLiteralName "HasSeenPlayer?") true))

(event OnComponentHit(RightLegHitbox)
  (params (HitComponent :type Primitive%20Component%20Object%20Reference) (OtherActor :type Actor%20Object%20Reference) (OtherComp :type Primitive%20Component%20Object%20Reference) (NormalImpulse :type Vector :default "0, 0, 0") (Hit :type Hit%20Result%20Structure%20%28by%20ref%29))
  ;[1 1 1] Shooting Score System Created
  (CallFunction|Ragdoll)
  (Utilities|FlowControl|Delay 1.0)
  (Actor|DestroyActor)
  (bind _asbp_first_person_game_mode (Utilities|Casting|CastToBP_FirstPersonGameMode (Game|GetGameMode)))
  (Default|ProjectileLegs _asbp_first_person_game_mode))

(event OnComponentHit(LeftLegHitbox)
  (params (HitComponent :type Primitive%20Component%20Object%20Reference) (OtherActor :type Actor%20Object%20Reference) (OtherComp :type Primitive%20Component%20Object%20Reference) (NormalImpulse :type Vector :default "0, 0, 0") (Hit :type Hit%20Result%20Structure%20%28by%20ref%29))
  ;[1 1 1] Shooting Score System Created
  (CallFunction|Ragdoll)
  (Utilities|FlowControl|Delay 1.0)
  (Actor|DestroyActor)
  (bind _asbp_first_person_game_mode (Utilities|Casting|CastToBP_FirstPersonGameMode (Game|GetGameMode)))
  (Default|ProjectileLegs _asbp_first_person_game_mode))

(event OnComponentHit(BodyLeftForearmHitBox)
  (params (HitComponent :type Primitive%20Component%20Object%20Reference) (OtherActor :type Actor%20Object%20Reference) (OtherComp :type Primitive%20Component%20Object%20Reference) (NormalImpulse :type Vector :default "0, 0, 0") (Hit :type Hit%20Result%20Structure%20%28by%20ref%29))
  ;[1 1 1] Shooting Score System Created
  (CallFunction|Ragdoll)
  (Utilities|FlowControl|Delay 1.0)
  (Actor|DestroyActor)
  (bind _asbp_first_person_game_mode (Utilities|Casting|CastToBP_FirstPersonGameMode (Game|GetGameMode)))
  (Default|ProjectileBody _asbp_first_person_game_mode))

(event OnComponentHit(BodyRightForearmHitBox)
  (params (HitComponent :type Primitive%20Component%20Object%20Reference) (OtherActor :type Actor%20Object%20Reference) (OtherComp :type Primitive%20Component%20Object%20Reference) (NormalImpulse :type Vector :default "0, 0, 0") (Hit :type Hit%20Result%20Structure%20%28by%20ref%29))
  ;[1 1 1] Shooting Score System Created
  (CallFunction|Ragdoll)
  (Utilities|FlowControl|Delay 1.0)
  (Actor|DestroyActor)
  (bind _asbp_first_person_game_mode (Utilities|Casting|CastToBP_FirstPersonGameMode (Game|GetGameMode)))
  (Default|ProjectileBody _asbp_first_person_game_mode))

(event OnComponentHit(BodyLeftArmHitBox)
  (params (HitComponent :type Primitive%20Component%20Object%20Reference) (OtherActor :type Actor%20Object%20Reference) (OtherComp :type Primitive%20Component%20Object%20Reference) (NormalImpulse :type Vector :default "0, 0, 0") (Hit :type Hit%20Result%20Structure%20%28by%20ref%29))
  ;[1 1 1] Shooting Score System Created
  (CallFunction|Ragdoll)
  (Utilities|FlowControl|Delay 1.0)
  (Actor|DestroyActor)
  (bind _asbp_first_person_game_mode (Utilities|Casting|CastToBP_FirstPersonGameMode (Game|GetGameMode)))
  (Default|ProjectileBody _asbp_first_person_game_mode))

(event OnComponentHit(BodyRightArmHitBox)
  (params (HitComponent :type Primitive%20Component%20Object%20Reference) (OtherActor :type Actor%20Object%20Reference) (OtherComp :type Primitive%20Component%20Object%20Reference) (NormalImpulse :type Vector :default "0, 0, 0") (Hit :type Hit%20Result%20Structure%20%28by%20ref%29))
  ;[1 1 1] Shooting Score System Created
  (CallFunction|Ragdoll)
  (Utilities|FlowControl|Delay 1.0)
  (Actor|DestroyActor)
  (bind _asbp_first_person_game_mode (Utilities|Casting|CastToBP_FirstPersonGameMode (Game|GetGameMode)))
  (Default|ProjectileBody _asbp_first_person_game_mode))

(event OnComponentHit(HeadHitBox)
  (params (HitComponent :type Primitive%20Component%20Object%20Reference) (OtherActor :type Actor%20Object%20Reference) (OtherComp :type Primitive%20Component%20Object%20Reference) (NormalImpulse :type Vector :default "0, 0, 0") (Hit :type Hit%20Result%20Structure%20%28by%20ref%29))
  ;[1 1 1] Shooting Score System Created
  (CallFunction|Ragdoll)
  (Utilities|FlowControl|Delay 1.0)
  (Actor|DestroyActor)
  (bind _asbp_first_person_game_mode (Utilities|Casting|CastToBP_FirstPersonGameMode (Game|GetGameMode)))
  (Default|ProjectileHead _asbp_first_person_game_mode))

(event OnComponentHit(BodyHitBox)
  (params (HitComponent :type Primitive%20Component%20Object%20Reference) (OtherActor :type Actor%20Object%20Reference) (OtherComp :type Primitive%20Component%20Object%20Reference) (NormalImpulse :type Vector :default "0, 0, 0") (Hit :type Hit%20Result%20Structure%20%28by%20ref%29))
  ;[1 1 1] Shooting Score System Created
  (CallFunction|Ragdoll)
  (Utilities|FlowControl|Delay 1.0)
  (Actor|DestroyActor)
  (bind _asbp_first_person_game_mode (Utilities|Casting|CastToBP_FirstPersonGameMode (Game|GetGameMode)))
  (Default|ProjectileBody _asbp_first_person_game_mode))

(event OnComponentHit(LeftLegUpHitbox)
  (params (HitComponent :type Primitive%20Component%20Object%20Reference) (OtherActor :type Actor%20Object%20Reference) (OtherComp :type Primitive%20Component%20Object%20Reference) (NormalImpulse :type Vector :default "0, 0, 0") (Hit :type Hit%20Result%20Structure%20%28by%20ref%29))
  ;[1 1 1] Shooting Score System Created
  (CallFunction|Ragdoll)
  (Utilities|FlowControl|Delay 1.0)
  (Actor|DestroyActor)
  (bind _asbp_first_person_game_mode (Utilities|Casting|CastToBP_FirstPersonGameMode (Game|GetGameMode)))
  (Default|ProjectileLegs _asbp_first_person_game_mode))

(event OnComponentHit(RightLegUpHitbox)
  (params (HitComponent :type Primitive%20Component%20Object%20Reference) (OtherActor :type Actor%20Object%20Reference) (OtherComp :type Primitive%20Component%20Object%20Reference) (NormalImpulse :type Vector :default "0, 0, 0") (Hit :type Hit%20Result%20Structure%20%28by%20ref%29))
  ;[1 1 1] Shooting Score System Created
  (CallFunction|Ragdoll)
  (Utilities|FlowControl|Delay 1.0)
  (Actor|DestroyActor)
  (bind _asbp_first_person_game_mode (Utilities|Casting|CastToBP_FirstPersonGameMode (Game|GetGameMode)))
  (Default|ProjectileLegs _asbp_first_person_game_mode))

(event Custom|Ragdoll
  ;[1 1 1] Ragdoll
  (Physics|SetSimulatePhysics (Variables|Character|GetMesh) true)
  (Pawn|Components|CharacterMovement|DisableMovement (Variables|Character|GetCharacterMovement)))

(event Custom|Shoot%20Player
  (bind _asbp_first_person_character (Utilities|Casting|CastToBP_FirstPersonCharacter (Game|Player|GetPlayerPawn 0)))
  (Transformation|SetActorRotation (Math|Rotator|FindRelativeLookatRotation (Math|Conversions|ToTransform(Vector) (Transformation|GetActorLocation _asbp_first_person_character)) (Transformation|GetActorLocation)))
  (if (Variables|Default|GetCanAttach?)
    (Game|SpawnActorfromClass "/Game/FirstPerson/Blueprints/BP_FirstPersonProjectile.BP_FirstPersonProjectile_C" (Transformation|GetWorldTransform (Variables|Default|GetSpawnProjectile)) "Undefined" 0 0)
    (Game|Damage|ApplyDamage _asbp_first_person_character 1.0 0 0)
    (Variables|Default|SetCanAttach? true)
    (Utilities|FlowControl|Delay 0.2)
    (Variables|Default|SetCanAttach? true)))

(event EventBeginPlay
  (bind _returnvalue (Game|SpawnActorfromClass "/Game/Gun/BP_Gun.BP_Gun_C" (Transformation|GetSocketTransform (Variables|Character|GetMesh) "RightHandSocket" "RTS_World") "Undefined" 0 0))
  (Transformation|AttachComponentToComponent _returnvalue (Variables|Character|GetMesh) "RightHandSocket" "SnapToTarget" "SnapToTarget" "SnapToTarget" true))

(fn ConstructionScript)