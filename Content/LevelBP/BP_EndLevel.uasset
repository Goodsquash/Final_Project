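; BP_EndLevel is a trigger actor that ends a level and teleports the player to the start of a new area.
; When the first-person character overlaps its Box, it clears all widgets, briefly shows the EndLevel widget, then replaces it with fresh Timer and Point widgets.
; After a short delay it moves the player to NewStart, whose location is relative to the actor while its rotation is applied as-is.
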(event OnComponentBeginOverlap(Box)
  (params (OverlappedComponent :type Primitive%20Component%20Object%20Reference) (OtherActor :type Actor%20Object%20Reference) (OtherComp :type Primitive%20Component%20Object%20Reference) (OtherBodyIndex :type Integer) (bFromSweep :type Boolean) (SweepResult :type Hit%20Result%20Structure%20%28by%20ref%29))
  (bind _newstart (Variables|Default|GetNewStart))
  ;[1 1 1] Starting new level teleporting player to new area
  (bind _asbp_first_person_character (Utilities|Casting|CastToBP_FirstPersonCharacter OtherActor))
  (Viewport|RemoveAllWidgets)
  (bind _returnvalue (UserInterface|CreateWidget "/Game/UI/EndLevel.EndLevel_C"))
  (UserInterface|Viewport|AddtoViewport _returnvalue 0)
  (Utilities|FlowControl|Delay 0.2)
  (Viewport|RemoveAllWidgets)
  (bind _returnvalue_2 (UserInterface|CreateWidget "/Game/UI/Timer.Timer_C"))
  (bind _returnvalue_3 (UserInterface|CreateWidget "/Game/UI/Point.Point_C"))
  (UserInterface|Viewport|AddtoViewport _returnvalue_2 0)
  (Utilities|FlowControl|Delay 1.0)
  (Transformation|SetActorLocationAndRotation _asbp_first_person_character (Math|Transform|TransformLocation (Transformation|GetActorTransform) (.location _newstart)) (.rotation _newstart))
  (Utilities|FlowControl|Delay 1.0))

(fn ConstructionScript)