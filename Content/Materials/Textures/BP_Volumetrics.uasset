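; BP_Volumetrics is an actor that fakes a volumetric effect by stacking mesh layers upward through a set height.
; On BeginPlay it gives the base Plane a dynamic material instance, then spawns static mesh components at evenly spaced Z offsets based on VolumeHeight and VolumeResolution.
; Every layer's material receives the base world Z and the volume height as MinFrom_BP and MaxFrom_BP parameters, so the shader knows the volume's vertical range.
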(event EventBeginPlay
  (bind _plane (Variables|Default|GetPlane))
  (bind _returnvalue (Transformation|GetWorldLocation _plane))
  (bind _returnvalue_2 (Rendering|Material|CreateDynamicMaterialInstance _plane 0 (Rendering|Material|GetMaterial _plane 0) "None" :!class /Script/Engine.PrimitiveComponent))
  (Variables|Default|SetSeed_Height (.z _returnvalue))
  (Rendering|Material|SetScalarParameterValue _returnvalue_2 "MinFrom_BP" (.z _returnvalue) :!class /Script/Engine.MaterialInstanceDynamic)
  (Rendering|Material|SetScalarParameterValue _returnvalue_2 "MaxFrom_BP" (Variables|Default|GetVolume_Height) :!class /Script/Engine.MaterialInstanceDynamic)
  (for _index (range 0 (Variables|Default|GetVolume_Resolution))
    (bind _returnvalue_3 (AddComponent|AddStaticMeshComponent false (Math|Transform|MakeTransform (Math|Vector|MakeVector 0.0 0.0 (Variables|Default|GetPrevious_Layer_Height)) "0, 0, 0" "1.000000,1.000000,1.000000")))
    (Variables|Default|SetPrevious_Layer_Height (+ (Variables|Default|GetPrevious_Layer_Height) (/ (Variables|Default|GetVolume_Height) (Variables|Default|GetVolume_Resolution))))
    (bind _returnvalue_4 (Rendering|Material|CreateDynamicMaterialInstance _returnvalue_3 0 (Rendering|Material|GetMaterial _returnvalue_3 0) "None" :!class /Script/Engine.PrimitiveComponent))
    (Rendering|Material|SetScalarParameterValue _returnvalue_4 "MinFrom_BP" (Variables|Default|GetSeed_Height) :!class /Script/Engine.MaterialInstanceDynamic)
    (Rendering|Material|SetScalarParameterValue _returnvalue_4 "MaxFrom_BP" (Variables|Default|GetVolume_Height) :!class /Script/Engine.MaterialInstanceDynamic)))

(fn ConstructionScript)